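; Player pawn built on the Mover plugin that adds dash, double jump, vault, crouch, aim-strafe and zipline abilities.
; Enhanced Input sets flags that are packed into Mover's input collection, then read each pre-simulation tick to queue layered moves and mode changes.
; Dashes play directional montages; vaults trace obstacles for lip, step and landing motion-warp targets while flying.
; Mode-change events track ziplining and grant air jumps when walking off ledges.
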(event `self.ReceiveBeginPlay`
  (bind _charactermotioncomponent (`self.CharacterMotionComponent`))
  (`|ExecutionSequence`
    (:`then_0`
      ; Bind to Mover Component Events
      (add `CharacterMoverComponent.OnStanceChanged` _charactermotioncomponent (`|CreateDelegate` :!event `OnStanceChanged_Event`))
      (add `MoverComponent.OnMovementModeChanged` _charactermotioncomponent (`|CreateDelegate` :!event `OnMovementModeChanged_Event`))
      (add `MoverComponent.OnPreSimulationTick` _charactermotioncomponent (`|CreateDelegate` :!event `OnPresimulationTick_Event`)))
    (:`then_1`
      (`KismetArrayLibrary.Array_Add` (`self.InputMappingContextsApplied`) "/MoverExamples/Input/Mappings/IMC_AdvancedMoverMappingContext.IMC_AdvancedMoverMappingContext"))
    (:`then_2`
      (`parent.ReceiveBeginPlay`))))

(event `OnPresimulationTick_Event`
  (params (TimeStep :type "MoverTimeStep Structure (by ref)") (InputCmd :type "MoverInputCmdContext Structure (by ref)"))
  (bind _inputcollection (break `MoverInputCmdContext` InputCmd))
  ;[0.4271 0.4271 0.4271] Directional Dashing: queue up a programmatic movement when we see dashing input in the simulation update
  (`|ExecutionSequence`
    (:`then_0`
      (bind (_didsucceed _targetasrawbytes) (`MoverDataCollectionLibrary.K2_GetDataFromCollection` _inputcollection))
      (if _didsucceed
        (set `self.MovementInputs` _targetasrawbytes)))
    (:`then_1`
      (bind (_didsucceed_2 _targetasrawbytes_2) (`MoverDataCollectionLibrary.K2_GetDataFromCollection` _inputcollection))
      (if _didsucceed_2
        (set `self.Ability Inputs` _targetasrawbytes_2)))
    (:`then_2`
      (`self.HandleCrouchInput`)
      (`self.HandleDoubleJumpInput`)
      (`self.HandleVaultOverInput`)
      (`self.HandleDashInput`)
      (`self.HandleAimingInput`))))

(event `OnMovementModeChanged_Event`
  (params (PreviousMovementModeName :type "Name (by ref)") (NewMovementModeName :type "Name (by ref)"))
  ;[0 1 0.8866] Listening to mode switch
  (`self.CheckDoubleJumpTransfer` PreviousMovementModeName NewMovementModeName)
  (`self.CheckZiplineTransfer` NewMovementModeName))

(event `OnStanceChanged_Event`
  (params (OldStance :type "EStanceMode Enum" :default "Invalid") (NewStance :type "EStanceMode Enum" :default "Invalid"))
  ;[0.4688 0 0.2667 0.5] On Stance Changed
  (`|ExecutionSequence`
    (:`then_0`
      (if (`|EnumEquality` OldStance "Crouch")
        (set `self.WantsToCrouch` false)))
    (:`then_1`
      (if (`|EnumEquality` NewStance "Crouch")
        (set `self.WantsToCrouch` true)))))

(event `HandleAimingInput`
  (bind (_bisdashjustpressed _bisaimpressed) (break `MoverExampleAbilityInputs` (`self.Ability Inputs`)))
  ;[1 0 0.7091] Set aiming/strafing based on input
  (set `self.bOrientRotationToMovement` (not _bisaimpressed))
  (set `self.ShouldStrafe` _bisaimpressed))

(event `EnhancedInput|/MoverExamples/Input/Actions/IA_Dash`
  (params (ActionValue :type Boolean) (ElapsedSeconds :type "Float (double-precision)") (TriggeredSeconds :type "Float (double-precision)") (InputAction :type "InputAction Object Reference" :default "/MoverExamples/Input/Actions/IA_Dash.IA_Dash"))
  ;[0.4271 0.4271 0.4271] Capture Dashing Inputs
  (:`Started`
    (set `self.IsDashJustPressed` (not (`self.IsDashPressed`)))
    (set `self.IsDashPressed` true))
  (:`Completed`
    (set `self.IsDashPressed` false)
    (set `self.IsDashJustPressed` false)))

(event `HandleDashInput`
  (bind _charactermotioncomponent (`self.CharacterMotionComponent`))
  (bind _dashmagnitude (`self.DashMagnitude`))
  (bind _returnvalue (`SceneComponent.GetForwardVector` (`self.Capsule`)))
  ;[0.3065 1 0.3381] Activate dashing action based on input - Note: Dash delay/cooldown is not rollback friendly and is currently only for this simple example
  (if (and (`.bIsDashJustPressed` (break `MoverExampleAbilityInputs` (`self.Ability Inputs`))) (> (`GameplayStatics.GetTimeSeconds`) (+ (`self.TimeOfLastDash`) (`self.DashCooldown`))))
    (bind _returnvalue_2 (`MoverDataModelBlueprintLibrary.GetMoveDirectionIntentFromInputs` (`self.MovementInputs`)))
    (if (> (`KismetMathLibrary.VSize` _returnvalue_2) 0.0)
      (set `self.TimeOfLastDash` (`GameplayStatics.GetTimeSeconds`))
      (bind (_directionalmontage _biasforwardmovement) (`self.SelectDirectionalMontage` _returnvalue _returnvalue_2))
      (`MoverComponent.K2_QueueLayeredMove` _charactermotioncomponent (make `LayeredMove_LinearVelocity` (* (select `bool` _biasforwardmovement :`false` _returnvalue_2 :`true` (* _returnvalue (1.0 1.0 1.2))) (`KismetMathLibrary.MakeVector` _dashmagnitude _dashmagnitude _dashmagnitude)) null 0 "OverrideVelocity" 0 (`self.DashDurationMs`) (make `LayeredMoveFinishVelocitySettings` (0.0 0.0 0.0) 1000.0 (select `bool` (`CharacterMoverComponent.IsOnGround` (`self.CharacterMotionComponent`)) :`false` "ClampVelocity" :`true` "MaintainLastRootMotionVelocity" :!type "ELayeredMoveFinishVelocityMode Enum"))))
      (set `self.IsDashing` true)
      (`|PlayMontageOnMoverActor` _charactermotioncomponent _directionalmontage
        (:`OnCompleted`
          (set `self.IsDashing` false))))))

(event `EnhancedInput|/MoverExamples/Input/Actions/IA_Crouch`
  (params (ActionValue :type Boolean) (ElapsedSeconds :type "Float (double-precision)") (TriggeredSeconds :type "Float (double-precision)") (InputAction :type "InputAction Object Reference" :default "/MoverExamples/Input/Actions/IA_Crouch.IA_Crouch"))
  ;[0.4072 0.4072 0.4072] Capture Crouching Input
  (:`Triggered`
    (set `self.WantsToCrouch` (not (`self.WantsToCrouch`)))))

(event `EnhancedInput|/MoverExamples/Input/Actions/IA_ADS`
  (params (ActionValue :type Boolean) (ElapsedSeconds :type "Float (double-precision)") (TriggeredSeconds :type "Float (double-precision)") (InputAction :type "InputAction Object Reference" :default "/MoverExamples/Input/Actions/IA_ADS.IA_ADS"))
  ;[1 1 1] Capture Aiming Inputs
  (:`Triggered`
    (set `self.IsAiming` true)
    (`SceneComponent.K2_SetRelativeLocation` (`self.Camera`) (`self.ZoomCameraLocation`) false false))
  (:`Completed`
    (set `self.IsAiming` false)
    (`SceneComponent.K2_SetRelativeLocation` (`self.Camera`) (`self.OriginalCameraLocation`) false false)))

(event `HandleVaultOverInput`
  (bind _motion_warping_component (`self.Motion Warping Component`))
  ;[0.3785 0.4775 1] Vaulting Action: attempt to find an obstacle in front of us and vault over it
  (if (and (`CharacterMoverComponent.IsOnGround` (`self.CharacterMotionComponent`)) (`.bIsVaultJustPressed` (break `MoverExampleAbilityInputs` (`self.Ability Inputs`))))
    (bind (_canvaultover _vaultoverlippos _vaultoversteppos _vaultoverlandpos) (`self.TryGetVaultOverParams`))
    (if _canvaultover
      (`/Engine/EditorBlueprintResources/StandardMacros.IsValid` (`self.Motion Warping Component`)
        (:`Is Valid`
          (`MotionWarpingComponent.AddOrUpdateWarpTargetFromLocation` (`self.Motion Warping Component`) "VaultStartPos" _vaultoverlippos)
          (`MotionWarpingComponent.AddOrUpdateWarpTargetFromLocation` (`self.Motion Warping Component`) "VaultStepPos" _vaultoversteppos)
          (`MotionWarpingComponent.AddOrUpdateWarpTargetFromLocation` (`self.Motion Warping Component`) "VaultLandingPos" _vaultoverlandpos))
        (:`Is Not Valid`
          _))
      (`MoverComponent.QueueNextMode` (`self.CharacterMotionComponent`) "Flying" false)
      (`|PlayMontageOnMoverActor` (`self.CharacterMotionComponent`) "/MoverExamples/Characters/Mannequins/Animations/Manny/VaultOver_Montage.VaultOver_Montage"
        (:`OnBlendOut`
          _)
        (:`OnInterrupted`
          _))
      (`/Engine/EditorBlueprintResources/StandardMacros.IsValid` _motion_warping_component
        (:`Is Valid`
          (`MotionWarpingComponent.RemoveAllWarpTargets` _motion_warping_component))
        (:`Is Not Valid`
          _))
      (`MoverComponent.QueueNextMode` (`self.CharacterMotionComponent`) "Walking" false))))

(event `EnhancedInput|/MoverExamples/Input/Actions/IA_Vault`
  (params (ActionValue :type Boolean) (ElapsedSeconds :type "Float (double-precision)") (TriggeredSeconds :type "Float (double-precision)") (InputAction :type "InputAction Object Reference" :default "/MoverExamples/Input/Actions/IA_Vault.IA_Vault"))
  ;[0.4271 0.4271 0.4271] Capture Vaulting Inputs
  (:`Started`
    (set `self.IsVaultJustPressed` (not (`self.IsVaultPressed`)))
    (set `self.IsVaultPressed` true))
  (:`Completed`
    (set `self.IsVaultPressed` false)
    (set `self.IsVaultJustPressed` false)))

(event `HandleDoubleJumpInput`
  ;[1 0.1845 0] Activate double-jump based on input - Note this handles jump input so we should turn off the option for the CharacterMovercomponent to handle jump (bHandleJump)
  (if (and (`.bIsJumpJustPressed` (break `CharacterDefaultInputs` (`self.MovementInputs`))) (`CharacterMoverComponent.IsOnGround` (`self.CharacterMotionComponent`)))
    (`self.DoubleJump`)
    ;;[0.07812 0.07812 0.07812 0.5] Cancelling crouch if it's active
    (`CharacterMoverComponent.UnCrouch` (`self.CharacterMotionComponent`))))

(event `DoubleJump`
  ;[1 0.1829 0] Make and Queue Double Jump
  (`MoverComponent.K2_QueueLayeredMove` (`self.CharacterMotionComponent`) (make `LayeredMove_MultiJump` (`self.MaxInAirJumps`))))

(event `EnhancedInput|/MoverExamples/Input/Actions/IA_StartZipline`
  (params (ActionValue :type Boolean) (ElapsedSeconds :type "Float (double-precision)") (TriggeredSeconds :type "Float (double-precision)") (InputAction :type "InputAction Object Reference" :default "/MoverExamples/Input/Actions/IA_StartZipline.IA_StartZipline"))
  ;[0.4271 0.4271 0.4271] Capture Ziplining Inputs
  (:`Started`
    (set `self.IsStartZipliningPressed` true))
  (:`Completed`
    (set `self.IsStartZipliningPressed` false)))

(event `HandleCrouchInput`
  (bind _charactermotioncomponent (`self.CharacterMotionComponent`))
  ;[0.01492 0.0625 0 0.5] Handle Crouching
  (if (`.bWantsToBeCrouched` (break `MoverExampleAbilityInputs` (`self.Ability Inputs`)))
    (`CharacterMoverComponent.Crouch` _charactermotioncomponent)
    (else
      (`CharacterMoverComponent.UnCrouch` _charactermotioncomponent))))

(fn `ApplyIMC`
  (params (Controller :type "PlayerController Object Reference"))
  (`parent.ApplyIMC` Controller)
  (`EnhancedInputSubsystemInterface.AddMappingContext` (pcsubsystem `EnhancedInputLocalPlayerSubsystem` Controller) "/MoverExamples/Input/Mappings/IMC_AdvancedMoverMappingContext.IMC_AdvancedMoverMappingContext" 0 (struct)))

(fn `CanInAirJump`
  (returns (CanJump :type Boolean))
  (bind (_didsucceed _targetasrawbytes) (`MoverComponent.K2_FindActiveLayeredMove` (`self.CharacterMotionComponent`)))
  (bind (_maximuminairjumps _upwardsspeed _jumpsinairremaining _timeoflastjumpms) (break `LayeredMove_MultiJump` _targetasrawbytes))
  (if (`CharacterMoverComponent.IsOnGround` (`self.CharacterMotionComponent`))
    (return false)
    (elif _didsucceed
      (if (and (!= _maximuminairjumps _jumpsinairremaining) (> _timeoflastjumpms (`self.TimeOfLastInAirJump`)))
        (set `self.TimeOfLastInAirJump` _timeoflastjumpms)
        (return true)
        (else
          (return false)))
      (else
        (return false)))))

(fn `CheckDoubleJumpTransfer`
  (params (OldModename :type Name) (NewModeName :type Name))
  ;[1 1 1] Listening to a switch from walking to falling - queueing a double jump so pawn can jump in air - layered move handles filtering out inital jump
  (if (and (== OldModename "Walking") (== NewModeName "Falling") (not (`.bIsJumpJustPressed` (break `CharacterDefaultInputs` (`self.MovementInputs`)))))
    (`self.DoubleJump`)))

(fn `CheckZiplineTransfer`
  (params (NewModeName :type Name))
  (set `self.IsZiplining` (== NewModeName "Ziplining")))

(fn `OnProduceInputInBlueprint`
  (params (DeltaMs :type "Float (single-precision)") (InputCmd :type "MoverInputCmdContext Structure"))
  (returns (ReturnValue :type "MoverInputCmdContext Structure"))
  (locals (ProducedAbilityInput :type "MoverExampleAbilityInputs Structure") (bWantsToCrouch :type Boolean))
  ;[0.3906 0.3906 0.3906] Add our pawn's movement inputs to the collection.   We are adding this every frame for simplicity, but a project might choose to NOT add it unless there is any action-causing input.
  (bind _output_get (set `local.ProducedAbilityInput` (make `MoverExampleAbilityInputs` (`self.IsDashJustPressed`) (`self.IsAiming`) (`self.IsVaultJustPressed`) (`self.IsStartZipliningPressed`) (`self.WantsToCrouch`))))
  (`MoverDataCollectionLibrary.K2_AddDataToCollection` (`.InputCollection` (break `MoverInputCmdContext` InputCmd)) _output_get)
  (`|ExecutionSequence`
    (:`then_0`
      (set `self.IsDashJustPressed` false))
    (:`then_1`
      (set `self.IsVaultJustPressed` false))
    (:`then_2`
      (return InputCmd))))

(fn `SelectDirectionalMontage`
  (params (FacingDirection :type "Vector Structure") (MovementDirection :type "Vector Structure"))
  (returns (DirectionalMontage :type "AnimMontage Object Reference") (BiasForwardMovement :type Boolean))
  (locals (MontageToPick :type "AnimMontage Object Reference") (BiasForward :type Boolean))
  (bind (_returnvalue_roll _returnvalue_pitch _returnvalue_yaw) (`KismetMathLibrary.BreakRotator` (`KismetMathLibrary.NormalizedDeltaRotator` (`KismetMathLibrary.Conv_VectorToRotator` MovementDirection) (`KismetMathLibrary.Conv_VectorToRotator` FacingDirection))))
  (bind _returnvalue (`KismetMathLibrary.Abs` _returnvalue_yaw))
  (if (< _returnvalue 45.0)
    (set `local.MontageToPick` (`self.ForwardDash`))
    (set `local.BiasForward` true)
    (else
      (if (> _returnvalue 135.0)
        (set `local.MontageToPick` (`self.BackwardsDash`))
        (elif (< _returnvalue_yaw 0.0)
          (set `local.MontageToPick` (`self.LeftDash`))
          (else
            (set `local.MontageToPick` (`self.RightDash`)))))
      (set `local.BiasForward` false)))
  (return (`local.MontageToPick`) (`local.BiasForward`)))

(fn `TryGetVaultOverParams`
  (returns (CanVaultOver :type Boolean) (VaultOverLipPos :type "Vector Structure") (VaultOverStepPos :type "Vector Structure") (VaultOverLandPos :type "Vector Structure"))
  (locals (ObstacleInitialHitPos :type "Vector Structure") (ObstacleLipPos :type "Vector Structure" :default (0.0 0.0 0.0)) (ObstacleStepPos :type "Vector Structure") (ObstacleLandPos :type "Vector Structure") (DidSetLipPos :type Boolean) (DidSetStepPos :type Boolean) (DidSetLandPos :type Boolean) (DidFindPotentialVaultObstacle :type Boolean))
  (bind (_returnvalue_x _returnvalue_y) (`KismetMathLibrary.BreakVector` (`self.K2_GetActorLocation`)))
  (bind (_returnvalue_x_2 _returnvalue_y_2 _returnvalue_z) (`KismetMathLibrary.BreakVector` (`self.K2_GetActorLocation`)))
  (bind (_returnvalue_x_3 _returnvalue_y_3 _returnvalue_z_2) (`KismetMathLibrary.BreakVector` (`self.K2_GetActorLocation`)))
  (bind (_returnvalue_x_4 _returnvalue_y_4 _returnvalue_z_3) (`KismetMathLibrary.BreakVector` (`self.K2_GetActorLocation`)))
  (bind _returnvalue (+ (`local.ObstacleStepPos`) (* (`self.GetActorForwardVector`) (/ (`self.MaxVaultoverTransitionDistance`) (`self.NumVaultOverSamples`)))))
  (`|ExecutionSequence`
    (:`then_0`
      ;[0.2656 0.2656 0.2656] 1: Find potential vaultable obstacle in front of us,  raytesting increasingly higher until we have a blocking hit
      (for _index (range 4)
        (bind _returnvalue_2 (`KismetMathLibrary.MakeVector` _returnvalue_x _returnvalue_y (+ (* (`KismetMathLibrary.Conv_IntToDouble` _index) (/ (- (`self.MaxVaultoverHeight`) (`self.MinVaultoverHeight`)) 3.0)) (+ (- _returnvalue_z_3 (`CapsuleComponent.CapsuleHalfHeight` (`self.Capsule`))) (`self.MinVaultoverHeight`)))))
        (bind (_outhit _returnvalue_3) (`KismetSystemLibrary.SphereTraceSingle` :`Start` _returnvalue_2 :`End` (+ _returnvalue_2 (* (`self.GetActorForwardVector`) (`self.MaxVaultoverStartDistance`))) :`Radius` 5.0 :`TraceChannel` "TraceTypeQuery1" :`DrawTime` 0.05))
        (if _returnvalue_3
          (`|ExecutionSequence`
            (:`then_0`
              (set `local.DidFindPotentialVaultObstacle` true)
              (set `local.ObstacleInitialHitPos` (`.Location` (`GameplayStatics.BreakHitResult` _outhit))))
            (:`then_1`
              (break))))))
    (:`then_1`
      ;[0.2667 0.2667 0.2667] 2: Perform downward traces along the forward line of the actor, increasingly farther into the obstacle
      (if (`local.DidFindPotentialVaultObstacle`)
        (for _index_2 (range (+ (`self.NumVaultOverSamples`) 1))
          (bind _returnvalue_4 (+ (* (`self.GetActorForwardVector`) (* _index_2 (/ (`self.MaxVaultoverTransitionDistance`) (`self.NumVaultOverSamples`)))) (`KismetMathLibrary.MakeVector` (.x (`local.ObstacleInitialHitPos`)) (.y (`local.ObstacleInitialHitPos`)) (- (+ (`self.MaxVaultoverHeight`) _returnvalue_z) (`CapsuleComponent.CapsuleHalfHeight` (`self.Capsule`))))))
          (bind (_outhit_2 _returnvalue_5) (`KismetSystemLibrary.SphereTraceSingle` :`Start` _returnvalue_4 :`End` (- _returnvalue_4 (`KismetMathLibrary.MakeVector` 0.0 0.0 (- (`self.MaxVaultoverHeight`) (`self.MinVaultoverHeight`)))) :`Radius` 10.0 :`TraceChannel` "TraceTypeQuery1" :`TraceHitColor` (struct :`R` 0.132995 :`G` 0.114583 :`B` 1.0 :`A` 1.0) :`DrawTime` 0.5))
          (if _returnvalue_5
            (bind (_bblockinghit _binitialoverlap _time _distance _location) (`GameplayStatics.BreakHitResult` _outhit_2))
            (if (and _bblockinghit (not _binitialoverlap))
              (`|ExecutionSequence`
                (:`then_0`
                  (if (== _index_2 0)
                    (bind _output_get (set `local.ObstacleLipPos` _location))
                    (set `local.DidSetLipPos` true)))
                (:`then_1`
                  (bind _output_get_2 (set `local.ObstacleStepPos` _location))
                  (set `local.DidSetStepPos` true)))
              (else
                (break)))
            (else
              (break))))))
    (:`then_2`
      ;[0.2667 0.2667 0.2667] 3:  Perform a final downward trace just past our last successful trace, but longer and looking for a landing point
      (if (and (`local.DidSetLipPos`) (`local.DidSetStepPos`))
        (bind (_outhit_3 _returnvalue_6) (`KismetSystemLibrary.LineTraceSingle` :`Start` _returnvalue :`End` (`KismetMathLibrary.MakeVector` (.x _returnvalue) (.y _returnvalue) (- _returnvalue_z_2 (* (`CapsuleComponent.CapsuleHalfHeight` (`self.Capsule`)) 2.0))) :`TraceChannel` "TraceTypeQuery1" :`TraceColor` (struct :`R` 0.599286 :`G` 1.0 :`A` 1.0) :`TraceHitColor` (struct :`R` 1.0 :`A` 1.0) :`DrawTime` 0.5))
        (bind (_bblockinghit_2 _binitialoverlap_2 _time_2 _distance_2 _location_2) (`GameplayStatics.BreakHitResult` _outhit_3))
        (if (and _returnvalue_6 (not _binitialoverlap_2))
          (set `local.ObstacleLandPos` _location_2)
          (set `local.DidSetLandPos` true))))
    (:`then_3`
      ;[0.2667 0.2667 0.2667] 4: Gather and return results
      (return (and (`local.DidFindPotentialVaultObstacle`) (`local.DidSetLipPos`) (`local.DidSetStepPos`) (`local.DidSetLandPos`)) (`local.ObstacleLipPos`) (`local.ObstacleStepPos`) (`local.ObstacleLandPos`)))))

(fn `UserConstructionScript`
  (`parent.UserConstructionScript`))